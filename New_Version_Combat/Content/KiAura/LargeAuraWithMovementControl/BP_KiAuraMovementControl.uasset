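; Ki aura controller that makes a large Niagara aura react to a character's movement.
; PrepareMaterialInstance creates a dynamic blinking-lightning material and assigns it to the supplied Niagara component.
; ProcessAuraMovement smoothly interpolates the aura offset against velocity direction, with an upward bias unless rising, and reverses spike flow when rising.
; It shows lightning only at standstill via a material layer parameter; both functions rely on external callers, as the event graph is empty.
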(event EventBeginPlay)

(event Collision|EventActorBeginOverlap
  (params (OtherActor :type Actor%20Object%20Reference)))

(event EventTick
  (params (DeltaSeconds :type Float%20%28single-precision%29)))

(fn ConstructionScript)

(fn PrepareMaterialInstance
  (params (TargetNiagaraComponent :type Niagara%20Component%20Object%20Reference%20%28by%20ref%29))
  (bind _returnvalue (Rendering|Material|CreateDynamicMaterialInstance "/Game/KiAura/LargeAuraWithMovementControl/Materials/MI_LargeAura_MovementControl_BlinkingLightning.MI_LargeAura_MovementControl_BlinkingLightning" "None" "None" :!class /Script/Engine.KismetMaterialLibrary))
  (bind _output_get (Variables|Default|SetMaterialInstance _returnvalue))
  (bind _output_get_2 (Variables|Default|SetMovingAura TargetNiagaraComponent))
  (Class|NiagaraComponent|SetVariableMaterial _output_get_2 "AuraMaterial" _output_get))

(fn ProcessAuraMovement
  (params (Character :type Character%20Object%20Reference))
  (bind _materialinstance (Variables|Default|GetMaterialInstance))
  (bind _movingaura (Variables|Default|GetMovingAura))
  (bind _returnvalue (Transformation|GetVelocity Character))
  (bind _returnvalue_2 (Math|Vector|Normalize _returnvalue))
  (bind _z (Class|KismetMathLibrary|BreakVector3f _returnvalue_2))
  (bind _returnvalue_3 (Math|Vector|VectorLength _returnvalue_2))
  (bind _returnvalue_4 (> _z 0.01))
  (bind _returnvalue_5 (< _returnvalue_3 0.01))
  (Utilities|IsValid _movingaura
    (:Is%20Valid
      (Utilities|IsValid (AssetData|GetAsset _movingaura)
        (:Is%20Valid
          (Variables|Default|SetisNotMoving _returnvalue_5)
          (Variables|Default|SetisGoingUp _returnvalue_4)
          ;[1 1 1] Smooth movement to target vector
          (bind _output_get (Variables|Default|SetauraOffset (Math|Interpolation|VInterpTo (stale _output_get) (+ (select _returnvalue_4 "0, 0, 0" (select _returnvalue_5 "0.000000,0.000000,1.000000" "0.000000,0.000000,0.500000")) (* _returnvalue_2 -1.0)) (Utilities|Time|GetWorldDeltaSeconds) 5.0)))
          (Niagara|SetNiagaraVariable(Vector3) (Variables|Default|GetMovingAura) "AuraWOffset" _output_get)
          (Utilities|IsValid _materialinstance
            (:Is%20Valid
              ;[1 1 1] Set opacity for lightning. Shows it only when not moving
              (Rendering|Material|SetScalarParameterValuebyInfo _materialinstance (Utilities|Struct|MakeMaterialParameterInfo "LightningOpacity" "LayerParameter" 1) (select (Variables|Default|GetisNotMoving) 3.0 0.0))
              ;[1 1 1] Changes spikes direction if is going up
              (Class|NiagaraComponent|SetVariableVec2 (Variables|Default|GetMovingAura) "AuraSpeed" (Math|Conversions|ToVector2D(Vector) (select (Variables|Default|GetisGoingUp) "0.000000,-2.000000,0.000000" "0.000000,2.000000,0.000000"))))))))))